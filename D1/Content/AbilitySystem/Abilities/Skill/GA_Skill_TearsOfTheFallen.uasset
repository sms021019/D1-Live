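; Gameplay ability for the Tears of the Fallen skill, which has the player pick a target with an AOE reticle.
; It extends the parent's WaitTargetData event with a user-confirmed targeting task that traces from the owner's head, configured by range, collision size and trace profile variables.
; Valid data is stored in TargetDataHandle and the ability commits before confirming the skill.
; A failed commit or cancelled targeting cancels the skill.
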(event EventWaitTargetData
  (|CallParentFunction)
  (bind _data (|WaitTargetData :TaskInstanceName "TargetDataTask" :ConfirmationType "UserConfirmed" :Class (Variables|Default|GetTargetActorClass) :CollisionRadius (Variables|Default|GetCollisionRadius) :CollisionHeight (Variables|Default|GetCollisionHeight) :MaxRange (Variables|Default|GetMaxRange) :TraceProfile (Variables|Default|GetTraceProfile) :StartLocation (Class|GameplayAbility|MakeTargetLocationInfofromOwnerSkeletalMeshComponent "head") :ReticleClass (Variables|Default|GetAOEReticleClass))
    (:ValidData
      (Variables|Default|SetTargetDataHandle _data)
      (bind _returnvalue (Ability|CommitAbility))
      (if _returnvalue
        (Class|D1GameplayAbilitySkillAOE|ConfirmSkill)
        (else
          (Class|D1GameplayAbilitySkillAOE|CancelSkill))))
    (:Cancelled
      (Class|D1GameplayAbilitySkillAOE|CancelSkill))))